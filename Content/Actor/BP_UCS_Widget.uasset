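; BP_UCS_Widget is an actor that displays a configurable widget through its Widget component.
; On BeginPlay it creates the widget from WidgetClass with Info, assigns it to the component and calls InitWidget.
; It then sets screen-space scale and pivot from the WidgetSize and WidgetPivot entries in Info's InfoMap.
; Its LogicInterface function prints the incoming InfoMap's Key entry, if present, and returns false.
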(event `self.ReceiveBeginPlay`
  (bind _infomap (break `UCS_LogicStruct` (`self.Info`)))
  (bind _returnvalue (`KismetStringLibrary.Conv_StringToDouble` (`BlueprintMapLibrary.Map_Find` _infomap "WidgetSize")))
  (bind _returnvalue_2 (`|CreateWidget` (`self.WidgetClass`) null (`self.Info`)))
  (`WidgetComponent.SetWidget` (`self.Widget`) _returnvalue_2)
  (`UCS_WidgetBase.InitWidget` _returnvalue_2)
  (`self.SetScreenSpaceWidgetScaleAndPivot` (`self.Widget`) (`KismetMathLibrary.MakeVector2D` _returnvalue _returnvalue) (`KismetStringLibrary.Conv_StringToVector2D` (`BlueprintMapLibrary.Map_Find` _infomap "WidgetPivot"))))

(fn `LogicInterface`
  (params (LogicInput :type "UCS_LogicStruct Structure"))
  (returns (ReturnValue :type Boolean))
  (bind (_value _returnvalue) (`BlueprintMapLibrary.Map_Find` (`.InfoMap` (break `UCS_LogicStruct` LogicInput)) "Key"))
  (if _returnvalue
    (`KismetSystemLibrary.PrintString` _value)
    (return false)))

(fn `UserConstructionScript`)